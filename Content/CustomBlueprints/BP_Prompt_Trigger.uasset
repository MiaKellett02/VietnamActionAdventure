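; BP_Prompt_Trigger is a box trigger that shows a text prompt on the player HUD while BP_Player stands inside it.
; It finds the W_PlayerHUD widget on BeginPlay, then sets the prompt on overlap begin and clears it on overlap end.
; UpdateUI pushes text to the HUD only when it differs from the last value.
; With ShowOnce set, the trigger stops responding after the first exit.
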(event `self.ReceiveBeginPlay`
  ;[1 1 1] Set Up the UI
  (bind _foundwidgets (`WidgetBlueprintLibrary.GetAllWidgetsOfClass` "/Game/UI/Widgets/W_PlayerHUD.W_PlayerHUD_C"))
  (bind _output_get (set `self.GameUI` (`|GetArrayItem` _foundwidgets)))
  (`/Game/UI/Widgets/W_PlayerHUD.UpdatePrompt` _output_get ""))

(event `self.Box.OnComponentBeginOverlap`
  (params (OverlappedComponent :type "PrimitiveComponent Object Reference") (OtherActor :type "Actor Object Reference") (OtherComp :type "PrimitiveComponent Object Reference") (OtherBodyIndex :type Integer) (bFromSweep :type Boolean) (SweepResult :type "HitResult Structure (by ref)"))
  ;[1 1 1] Set the prompt text when the player enters the prompt area.
  (if (not (`self.hasShown`))
    (cast `/Game/Blueprints/BP_Player` OtherActor)
    (set `self.NewText` (`self.PromptText`))
    (`self.UpdateUI`)))

(event `self.Box.OnComponentEndOverlap`
  (params (OverlappedComponent :type "PrimitiveComponent Object Reference") (OtherActor :type "Actor Object Reference") (OtherComp :type "PrimitiveComponent Object Reference") (OtherBodyIndex :type Integer))
  ;[1 1 1] Clear the prompt text when the player exits the prompt area.
  (if (not (`self.hasShown`))
    (cast `/Game/Blueprints/BP_Player` OtherActor)
    (set `self.NewText` "")
    (`self.UpdateUI`)
    (if (`self.ShowOnce`)
      (set `self.hasShown` true))))

(fn `UpdateUI`
  ;[1 1 1] Check if the text to display has changed.
  (if (not (`KismetTextLibrary.EqualEqual_TextText` (`self.NewText`) (`self.LastText`)))
    ;[1 1 1] If text has changed update UI
    (`/Game/UI/Widgets/W_PlayerHUD.UpdatePrompt` (`self.GameUI`) (`self.NewText`))
    (set `self.LastText` (`self.NewText`))))

(fn `UserConstructionScript`)