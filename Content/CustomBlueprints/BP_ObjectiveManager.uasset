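; Objective manager that walks the player through a linear mission: collect plane intel, destroy an AA, hijack a radio tower, then a placeholder completion message.
; Overlap triggers at the plane, AA and radio tower each advance the objective index, only when their step is current.
; UpdateUI maps the index to hard-coded text, which is sent to the W_PlayerHUD widget found on BeginPlay.
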(event `self.ReceiveBeginPlay`
  (set `self.objectiveIndex` 1)
  (bind _foundwidgets (`WidgetBlueprintLibrary.GetAllWidgetsOfClass` "/Game/UI/Widgets/W_PlayerHUD.W_PlayerHUD_C"))
  (set `self.GameUI` (`|GetArrayItem` _foundwidgets))
  (bind _newparam1 (`self.UpdateUI` 1))
  (`/Game/UI/Widgets/W_PlayerHUD.UpdateObjective` (`self.GameUI`) _newparam1)
  (set `self.objectiveIndex` 1))

(event `self.PlaneTrigger.OnComponentBeginOverlap`
  (params (OverlappedComponent :type "PrimitiveComponent Object Reference") (OtherActor :type "Actor Object Reference") (OtherComp :type "PrimitiveComponent Object Reference") (OtherBodyIndex :type Integer) (bFromSweep :type Boolean) (SweepResult :type "HitResult Structure (by ref)"))
  (if (== (`self.objectiveIndex`) 1)
    (`/Engine/EditorBlueprintResources/StandardMacros.IncrementInt` (`self.objectiveIndex`)
      (:`  `
        (bind _newparam1 (`self.UpdateUI` (`self.objectiveIndex`)))
        (`/Game/UI/Widgets/W_PlayerHUD.UpdateObjective` (`self.GameUI`) _newparam1)))))

(event `self.AATrigger.OnComponentBeginOverlap`
  (params (OverlappedComponent :type "PrimitiveComponent Object Reference") (OtherActor :type "Actor Object Reference") (OtherComp :type "PrimitiveComponent Object Reference") (OtherBodyIndex :type Integer) (bFromSweep :type Boolean) (SweepResult :type "HitResult Structure (by ref)"))
  (if (== (`self.objectiveIndex`) 2)
    (`/Engine/EditorBlueprintResources/StandardMacros.IncrementInt` (`self.objectiveIndex`)
      (:`  `
        (bind _newparam1 (`self.UpdateUI` (`self.objectiveIndex`)))
        (`/Game/UI/Widgets/W_PlayerHUD.UpdateObjective` (`self.GameUI`) _newparam1)))))

(event `self.RadioTrigger.OnComponentBeginOverlap`
  (params (OverlappedComponent :type "PrimitiveComponent Object Reference") (OtherActor :type "Actor Object Reference") (OtherComp :type "PrimitiveComponent Object Reference") (OtherBodyIndex :type Integer) (bFromSweep :type Boolean) (SweepResult :type "HitResult Structure (by ref)"))
  (if (== (`self.objectiveIndex`) 3)
    (`/Engine/EditorBlueprintResources/StandardMacros.IncrementInt` (`self.objectiveIndex`)
      (:`  `
        (bind _newparam1 (`self.UpdateUI` (`self.objectiveIndex`)))
        (`/Game/UI/Widgets/W_PlayerHUD.UpdateObjective` (`self.GameUI`) _newparam1)))))

(fn `UpdateUI`
  (params (Index :type Integer))
  (returns (NewParam1 :type Text))
  (locals (textReturn :type Text))
  (if (== Index 1)
    (set `local.textReturn` "Objective: \n1. Collect intel from plane")
    (return (`local.textReturn`))
    (elif (== Index 2)
      (set `local.textReturn` "Objective: \n2. Destroy that AA")
      (return (`local.textReturn`))
      (elif (== Index 3)
        (set `local.textReturn` "Objective: \n3. Hijack that radio tower")
        (return (`local.textReturn`))
        (elif (== Index 4)
          (set `local.textReturn` "GAME COMPLETE \nNEED TO ADD CUTSCENE")
          (else
            (return (`local.textReturn`))))))))

(fn `UserConstructionScript`)