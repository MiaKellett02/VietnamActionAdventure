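; BP_Door is a sliding door that players open by pressing Interact and that guard enemies open automatically.
; A trigger box enables the door's input while BP_Player overlaps it, and plays the DoorOpen timeline as soon as a BP_GuardEnemy enters.
; The timeline drives the door mesh's relative location.
; Either character leaving reverses it, without checking who remains inside.
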(event `self.TriggerBox.OnComponentBeginOverlap`
  (params (OverlappedComponent :type "PrimitiveComponent Object Reference") (OtherActor :type "Actor Object Reference") (OtherComp :type "PrimitiveComponent Object Reference") (OtherBodyIndex :type Integer) (bFromSweep :type Boolean) (SweepResult :type "HitResult Structure (by ref)"))
  (cast `/Game/Blueprints/BP_Player` OtherActor
    (:`then`
      (`self.EnableInput` (`GameplayStatics.GetPlayerController` 0)))
    (:`CastFailed`
      (cast `/Game/Blueprints/GuardCharacter/BP_GuardEnemy` OtherActor)
      (bind (_direction _doorslide) (`Timeline|DoorOpen` :!label _label)
        (:`Update`
          (`SceneComponent.K2_SetRelativeLocation` (`self.Door`) _doorslide false false))))))

(event `InputAction|Interact`
  (params (Key :type "Key Structure"))
  (:`Pressed`
    (goto _label)))

(event `self.TriggerBox.OnComponentEndOverlap`
  (params (OverlappedComponent :type "PrimitiveComponent Object Reference") (OtherActor :type "Actor Object Reference") (OtherComp :type "PrimitiveComponent Object Reference") (OtherBodyIndex :type Integer))
  (cast `/Game/Blueprints/BP_Player` OtherActor
    (:`then`
      (`self.DisableInput` (`GameplayStatics.GetPlayerController` 0))
      (goto _label :!via `Reverse`))
    (:`CastFailed`
      (cast `/Game/Blueprints/GuardCharacter/BP_GuardEnemy` OtherActor)
      (goto _label :!via `Reverse`))))

(fn `UserConstructionScript`)